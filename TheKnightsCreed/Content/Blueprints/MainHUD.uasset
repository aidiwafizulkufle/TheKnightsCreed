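; MainHUD is the bootstrap Blueprint that creates the on-screen HUD and the player's inventory manager.
; On BeginPlay it adds a WBP_HUD widget to the viewport and spawns a BP_InventoryManager at the world origin.
; It casts player 0's pawn to Player, assigns the manager, runs its Setup with the widget, and gives the Player a reference to that widget.
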(event `self.ReceiveBeginPlay`
  (bind _returnvalue (`|CreateWidget` "/Game/Blueprints/WBP_HUD.WBP_HUD_C"))
  (bind _output_get (set `self.HUDWidget` _returnvalue))
  (`UserWidget.AddToViewport` _returnvalue 0)
  (bind _returnvalue_2 (`|SpawnActorFromClass` "/Game/Blueprints/UI/InventorySystem/BP_InventoryManager.BP_InventoryManager_C" (`KismetMathLibrary.MakeTransform` (0.0 0.0 0.0)) "Undefined" "OverrideRootScale" null null))
  (bind _asplayer (cast `/Game/Blueprints/Player` (`Controller.K2_GetPawn` (`GameplayStatics.GetPlayerController` 0))))
  (bind _output_get_2 (set `/Game/Blueprints/Player.InventoryManager` _returnvalue_2 _asplayer))
  (`/Game/Blueprints/UI/InventorySystem/BP_InventoryManager.Setup` _output_get_2 _output_get)
  (set `/Game/Blueprints/Player.HudWidget` _returnvalue _asplayer))

(fn `UserConstructionScript`)