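; Base enemy character that patrols between two points, hurts the player on contact and ragdolls when its health runs out.
; Both point components detach at BeginPlay to stay fixed in the world, and Tick walks toward the current one, alternating via FlipFlop on arrival.
; Capsule hits damage the player and launch them upward and away along Y.
; A custom damage event clamps health and triggers death, while AnyDamage only calls the parent.
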(event `CustomEvent`
  (params (Damage :type "Float (double-precision)") (DamageType :type "DamageType Object Reference") (InstigatedBy :type "Controller Object Reference") (DamageCauser :type "Actor Object Reference"))
  ;[1 1 1] Take Damage
  (bind _output_get (set `self._currentHealth` (`KismetMathLibrary.FClamp` (- (`self._currentHealth`) Damage) 0.0 (`self.health`))))
  (if (<= _output_get 0.0)
    (`self.Die`)))

(event `Die`
  (bind _mesh (`self.Mesh`))
  ;[1 1 1] Death
  (`PrimitiveComponent.SetCollisionEnabled` _mesh "QueryAndPhysics")
  (`PrimitiveComponent.SetSimulatePhysics` _mesh true)
  (`SkeletalMeshComponent.SetPhysicsBlendWeight` _mesh 1.0))

(event `self.ReceiveBeginPlay`
  (`SceneComponent.K2_DetachFromComponent` (`self.point_2`) "KeepWorld" "KeepWorld" "KeepWorld" true)
  (`SceneComponent.K2_DetachFromComponent` (`self.point_1`) "KeepWorld" "KeepWorld" "KeepWorld" true)
  (`self.SetPatrolPoint`))

(event `self.ReceiveAnyDamage`
  (params (Damage :type "Float (single-precision)") (DamageType :type "DamageType Object Reference") (InstigatedBy :type "Controller Object Reference") (DamageCauser :type "Actor Object Reference"))
  (`parent.ReceiveAnyDamage` Damage DamageType InstigatedBy DamageCauser))

(event `self.ReceiveTick`
  (params (DeltaSeconds :type "Float (single-precision)"))
  (bind _returnvalue (`self.K2_GetActorLocation`))
  (bind _target_patrol_point (`self.target patrol point`))
  (if (`self.patrolling enabled`)
    (`self.AddMovementInput` (`KismetMathLibrary.GetDirectionUnitVector` _returnvalue _target_patrol_point) 0.3)
    (if (< (`KismetMathLibrary.Vector_Distance` _returnvalue _target_patrol_point) 100.0)
      (`self.SetPatrolPoint`))))

(event `SetPatrolPoint`
  (`/Engine/EditorBlueprintResources/StandardMacros.FlipFlop`
    (:`A`
      (set `self.target patrol point` (`SceneComponent.K2_GetComponentLocation` (`self.point_1`))))
    (:`B`
      (set `self.target patrol point` (`SceneComponent.K2_GetComponentLocation` (`self.point_2`))))))

(event `self.CapsuleComponent.OnComponentHit`
  (params (HitComponent :type "PrimitiveComponent Object Reference") (OtherActor :type "Actor Object Reference") (OtherComp :type "PrimitiveComponent Object Reference") (NormalImpulse :type "Vector Structure") (Hit :type "HitResult Structure (by ref)"))
  (bind (_returnvalue_x _returnvalue_y) (`KismetMathLibrary.BreakVector` (`self.K2_GetActorLocation`)))
  ;[1 1 1] KnockBack
  (bind _asplayer (cast `/Game/Blueprints/Player` OtherActor))
  (`GameplayStatics.ApplyDamage` _asplayer (`self.knockbackDamage`))
  (bind (_returnvalue_x_2 _returnvalue_y_2) (`KismetMathLibrary.BreakVector` (`self.K2_GetActorLocation` _asplayer)))
  (bind _returnvalue (* (`KismetMathLibrary.SignOfFloat` (- _returnvalue_y_2 _returnvalue_y)) (`self.playerKnockbackForce`)))
  (`self.LaunchCharacter` _asplayer (`KismetMathLibrary.MakeVector` 0.0 _returnvalue (`KismetMathLibrary.Abs` _returnvalue)) false false))

(fn `UserConstructionScript`
  (`parent.UserConstructionScript`)
  (set `self._currentHealth` (`self.health`)))