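; Base enemy Blueprint that handles damage and death by ragdoll.
; The AnyDamage event subtracts damage from CurrentHealth, clamped between zero and Health, and calls Death whenever the result is zero.
; Death enables query and physics collision on the mesh and switches it to fully blended physics simulation.
; No guard prevents Death from firing again on later hits.
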(event `self.ReceiveAnyDamage`
  (params (Damage :type "Float (single-precision)") (DamageType :type "DamageType Object Reference") (InstigatedBy :type "Controller Object Reference") (DamageCauser :type "Actor Object Reference"))
  ;[1 1 1] Take Damage
  (bind _output_get (set `self._currentHealth` (`KismetMathLibrary.FClamp` (- (`self._currentHealth`) Damage) 0.0 (`self.health`))))
  (if (<= _output_get 0.0)
    (`self.Death`)))

(event `Death`
  (bind _mesh (`self.Mesh`))
  ;[1 1 1] Death
  (`PrimitiveComponent.SetCollisionEnabled` _mesh "QueryAndPhysics")
  (`PrimitiveComponent.SetSimulatePhysics` _mesh true)
  (`SkeletalMeshComponent.SetPhysicsBlendWeight` _mesh 1.0))

(fn `UserConstructionScript`)