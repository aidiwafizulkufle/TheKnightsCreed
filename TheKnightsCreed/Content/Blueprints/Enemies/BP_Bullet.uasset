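; Enemy projectile that flies straight along its local X axis and hurts the player on contact.
; Tick moves it by ForwardSpeed scaled by delta time, without a movement component.
; Sphere overlap with a Player applies Damage and launches the character away along world Y and upward, both scaled by PlayerKnockbackForce.
; The graph never destroys the bullet, on hit or otherwise.
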(event `self.ReceiveTick`
  (params (DeltaSeconds :type "Float (single-precision)"))
  (`self.K2_AddActorLocalOffset` (`KismetMathLibrary.MakeVector` (* DeltaSeconds (`self.forwardSpeed`)))))

(event `self.Sphere.OnComponentBeginOverlap`
  (params (OverlappedComponent :type "PrimitiveComponent Object Reference") (OtherActor :type "Actor Object Reference") (OtherComp :type "PrimitiveComponent Object Reference") (OtherBodyIndex :type Integer) (bFromSweep :type Boolean) (SweepResult :type "HitResult Structure (by ref)"))
  (bind (_returnvalue_x _returnvalue_y) (`KismetMathLibrary.BreakVector` (`self.K2_GetActorLocation`)))
  ;[1 1 1] KnockBack
  (bind _asplayer (cast `/Game/Blueprints/Player` OtherActor))
  (`GameplayStatics.ApplyDamage` _asplayer (`self.damage`))
  (bind (_returnvalue_x_2 _returnvalue_y_2) (`KismetMathLibrary.BreakVector` (`self.K2_GetActorLocation` _asplayer)))
  (bind _returnvalue (* (`KismetMathLibrary.SignOfFloat` (- _returnvalue_y_2 _returnvalue_y)) (`self.playerKnockbackForce`)))
  (`Character.LaunchCharacter` _asplayer (`KismetMathLibrary.MakeVector` 0.0 _returnvalue (`KismetMathLibrary.Abs` _returnvalue)) false false))

(fn `UserConstructionScript`)