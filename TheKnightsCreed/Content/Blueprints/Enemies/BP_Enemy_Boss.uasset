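; BP_Enemy_Boss is a knife-wielding boss enemy built on a parent enemy Blueprint.
; On BeginPlay it spawns a BP_Knife and attaches it to a mesh socket.
; Overlapping the melee trigger plays a stab montage, then after a short delay damages the player with the knife's damage and launches them away along Y and upward.
; When health runs out, it destroys the knife and shows the player's restart display.
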(event `self.ReceiveBeginPlay`
  (bind _mesh (`self.Mesh`))
  (`parent.ReceiveBeginPlay`)
  (bind _returnvalue (`|SpawnActorFromClass` "/Game/Blueprints/Enemies/BP_Knife.BP_Knife_C" (`SceneComponent.GetSocketTransform` _mesh "knifeSocket" "RTS_World") "Undefined" "OverrideRootScale" null null))
  (set `self.Knife` _returnvalue)
  (`self.K2_AttachToComponent` _returnvalue _mesh "knifeSocket" "SnapToTarget" "SnapToTarget" "SnapToTarget" true))

(event `self.MeleeTrigger.OnComponentBeginOverlap`
  (params (OverlappedComponent :type "PrimitiveComponent Object Reference") (OtherActor :type "Actor Object Reference") (OtherComp :type "PrimitiveComponent Object Reference") (OtherBodyIndex :type Integer) (bFromSweep :type Boolean) (SweepResult :type "HitResult Structure (by ref)"))
  (bind (_returnvalue_x _returnvalue_y) (`KismetMathLibrary.BreakVector` (`self.K2_GetActorLocation`)))
  (bind _asplayer (cast `/Game/Blueprints/Player` OtherActor))
  (`|PlayMontage` (`self.Mesh`) "/Game/Models/Mixamo/StabMontage.StabMontage"
    (:`then`
      (`KismetSystemLibrary.Delay` 0.3)
      (`GameplayStatics.ApplyDamage` _asplayer (`/Game/Blueprints/Enemies/BP_Knife.Damage` (`self.Knife`)))
      (bind (_returnvalue_x_2 _returnvalue_y_2) (`KismetMathLibrary.BreakVector` (`self.K2_GetActorLocation` _asplayer)))
      (bind _returnvalue (* (`KismetMathLibrary.SignOfFloat` (- _returnvalue_y_2 _returnvalue_y)) (`self.playerKnockbackForce`)))
      (`self.LaunchCharacter` _asplayer (`KismetMathLibrary.MakeVector` 0.0 _returnvalue (`KismetMathLibrary.Abs` _returnvalue)) false false))))

(event `self.ReceiveAnyDamage`
  (params (Damage :type "Float (single-precision)") (DamageType :type "DamageType Object Reference") (InstigatedBy :type "Controller Object Reference") (DamageCauser :type "Actor Object Reference"))
  (`parent.ReceiveAnyDamage` Damage null null null)
  (if (<= (`self._currentHealth`) 0.0)
    (`self.K2_DestroyActor` (`self.Knife`))
    (bind _asplayer (cast `/Game/Blueprints/Player` (`GameplayStatics.GetPlayerPawn` 0)))
    (`/Game/Blueprints/Player.DisplayRestart` _asplayer)))

(fn `UserConstructionScript`
  (`parent.UserConstructionScript`))