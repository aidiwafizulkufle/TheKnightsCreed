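; BP_Enemy_Shooter is an enemy that continuously fires BP_Bullet projectiles.
; Tick calls its parent, then runs through a half-second Delay, which throttles spawning to roughly two bullets per second.
; Each bullet spawns at the BulletSpawnPoint location and gets a Direction of plus or minus one from the sign of the enemy's yaw, with no aiming or target check.
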(event `self.ReceiveTick`
  (params (DeltaSeconds :type "Float (single-precision)"))
  (bind (_returnvalue_roll _returnvalue_pitch _returnvalue_yaw) (`KismetMathLibrary.BreakRotator` (`self.K2_GetActorRotation`)))
  (bind _returnvalue_location (`KismetMathLibrary.BreakTransform` (`SceneComponent.K2_GetComponentToWorld` (`self.BulletSpawnPoint`))))
  (`parent.ReceiveTick` DeltaSeconds)
  (`KismetSystemLibrary.Delay` 0.5)
  (bind _returnvalue (`|SpawnActorFromClass` "/Game/Blueprints/Enemies/BP_Bullet.BP_Bullet_C" (`KismetMathLibrary.MakeTransform` _returnvalue_location) "Undefined" "OverrideRootScale" null null))
  (set `/Game/Blueprints/Enemies/BP_Bullet.direction` (`KismetMathLibrary.SelectFloat` 1.0 -1.0 (>= _returnvalue_yaw 0.0)) _returnvalue))

(fn `UserConstructionScript`
  (`parent.UserConstructionScript`))