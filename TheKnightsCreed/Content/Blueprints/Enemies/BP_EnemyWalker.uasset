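; BP_EnemyWalker is a walking enemy that patrols back and forth between two points, Point1 and Point2.
; On BeginPlay it detaches both point components with world transforms kept, so they stay fixed while the enemy moves.
; While patrolling is enabled, Tick applies scaled-down movement input toward the target and uses a FlipFlop to switch points on close approach.
; Damage handling passes straight to the parent class.
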(event `self.ReceiveBeginPlay`
  (`SceneComponent.K2_DetachFromComponent` (`self.point_2`) "KeepWorld" "KeepWorld" "KeepWorld" true)
  (`SceneComponent.K2_DetachFromComponent` (`self.point_1`) "KeepWorld" "KeepWorld" "KeepWorld" true)
  (`self.SetPatrolPoint`))

(event `self.ReceiveAnyDamage`
  (params (Damage :type "Float (single-precision)") (DamageType :type "DamageType Object Reference") (InstigatedBy :type "Controller Object Reference") (DamageCauser :type "Actor Object Reference"))
  (`parent.ReceiveAnyDamage` Damage DamageType InstigatedBy DamageCauser))

(event `self.ReceiveTick`
  (params (DeltaSeconds :type "Float (single-precision)"))
  (bind _returnvalue (`self.K2_GetActorLocation`))
  (bind _target_patrol_point (`self.target patrol point`))
  (if (`self.patrolling enabled`)
    (`self.AddMovementInput` (`KismetMathLibrary.GetDirectionUnitVector` _returnvalue _target_patrol_point) 0.3)
    (if (< (`KismetMathLibrary.Vector_Distance` _returnvalue _target_patrol_point) 100.0)
      (`self.SetPatrolPoint`))))

(event `SetPatrolPoint`
  (`/Engine/EditorBlueprintResources/StandardMacros.FlipFlop`
    (:`A`
      (set `self.target patrol point` (`SceneComponent.K2_GetComponentLocation` (`self.point_1`))))
    (:`B`
      (set `self.target patrol point` (`SceneComponent.K2_GetComponentLocation` (`self.point_2`))))))

(fn `UserConstructionScript`
  (`parent.UserConstructionScript`))