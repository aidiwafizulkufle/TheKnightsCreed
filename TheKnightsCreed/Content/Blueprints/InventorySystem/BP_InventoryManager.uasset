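; Inventory manager that tracks item counts and shows them in five HUD slot widgets supplied through Setup.
; AddItem counts items by name in a map, updating the matching slot or filling the first empty one.
; With no empty slot, a new item is still counted but not shown.
; EnableSlot checks the chosen slot's background and unchecks the rest, while BeginPlay only casts the HUD.
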(event `self.ReceiveBeginPlay`
  (cast `/Game/Blueprints/MainHUD` (`PlayerController.GetHUD` (`GameplayStatics.GetPlayerController` 0))))

(fn `Add Item`
  (params (ItemDetails :type "/Game/Blueprints/InventorySystem/ItemDetails Structure"))
  (bind _itemname (break `/Game/Blueprints/InventorySystem/ItemDetails` ItemDetails))
  (bind _itemdict (`self.ItemDict`))
  (bind _slots (`self.Slots`))
  (if (`BlueprintMapLibrary.Map_Contains` (`self.ItemDict`) _itemname)
    (`BlueprintMapLibrary.Map_Add` _itemdict _itemname (+ (`BlueprintMapLibrary.Map_Find` _itemdict _itemname) 1))
    (for _array_element _slots
      (bind _item_itemname (break `/Game/Blueprints/InventorySystem/ItemDetails` (`/Game/Blueprints/InventorySystem/WBP_InvSlot.Item` _array_element)))
      (if (`KismetStringLibrary.EqualEqual_StrStr` _item_itemname _itemname)
        (`/Game/Blueprints/InventorySystem/WBP_InvSlot.UpdateUI` _array_element (`BlueprintMapLibrary.Map_Find` (`self.ItemDict`) _item_itemname))
        (break)))
    (else
      (`BlueprintMapLibrary.Map_Add` _itemdict _itemname 1)
      (for _array_element_2 _slots
        (bind _item_itemname_2 (break `/Game/Blueprints/InventorySystem/ItemDetails` (`/Game/Blueprints/InventorySystem/WBP_InvSlot.Item` _array_element_2)))
        (if (`KismetStringLibrary.EqualEqual_StrStr` _item_itemname_2)
          (set `/Game/Blueprints/InventorySystem/WBP_InvSlot.Item` ItemDetails _array_element_2)
          (`/Game/Blueprints/InventorySystem/WBP_InvSlot.UpdateUI` _array_element_2 1)
          (break))))))

(fn `EnableSlot`
  (params (SlotIndex :type Integer))
  (for (_array_element _array_index) (`self.Slots`)
    (if (== _array_index SlotIndex)
      (bind _slotbg (`/Game/Blueprints/InventorySystem/WBP_InvSlot.SlotBG` _array_element))
      (`CheckBox.SetCheckedState` _slotbg "Checked")
      (else
        (`CheckBox.SetCheckedState` _slotbg "Unchecked")))))

(fn `Setup`
  (params (HUD :type "/Game/Blueprints/WBP_HUD Object Reference"))
  (set `self.Slots` (`|MakeArray` (`/Game/Blueprints/WBP_HUD.WBP_InvSlot_1` HUD) (`/Game/Blueprints/WBP_HUD.WBP_InvSlot_2` HUD) (`/Game/Blueprints/WBP_HUD.WBP_InvSlot_3` HUD) (`/Game/Blueprints/WBP_HUD.WBP_InvSlot_4` HUD) (`/Game/Blueprints/WBP_HUD.WBP_InvSlot_5` HUD)))
  (set `self.MainHUD` HUD))

(fn `UserConstructionScript`)