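; BP_PickupBase is an inventory pickup actor that is collected when the player overlaps its Box.
; On overlap it casts to Player and looks up the item's name in the InventoryManager's ItemDict.
; If the held value is below the MaxAmount in ItemDetails, it passes ItemDetails to AddItem and destroys itself; otherwise it stays in the world.
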(event `self.Box.OnComponentBeginOverlap`
  (params (OverlappedComponent :type "PrimitiveComponent Object Reference") (OtherActor :type "Actor Object Reference") (OtherComp :type "PrimitiveComponent Object Reference") (OtherBodyIndex :type Integer) (bFromSweep :type Boolean) (SweepResult :type "HitResult Structure (by ref)"))
  (bind (_itemdetails_itemname _itemdetails_itemimage _itemdetails_maxamount) (break `/Game/Blueprints/InventorySystem/ItemDetails` (`self.ItemDetails`)))
  (bind _asplayer (cast `/Game/Blueprints/Player` OtherActor))
  (if (< (`BlueprintMapLibrary.Map_Find` (`/Game/Blueprints/InventorySystem/BP_InventoryManager.ItemDict` (`/Game/Blueprints/Player.InventoryManager` _asplayer)) _itemdetails_itemname) _itemdetails_maxamount)
    (`/Game/Blueprints/InventorySystem/BP_InventoryManager.Add Item` (`/Game/Blueprints/Player.InventoryManager` _asplayer) (`self.ItemDetails`))
    (`self.K2_DestroyActor`)))

(fn `UserConstructionScript`)