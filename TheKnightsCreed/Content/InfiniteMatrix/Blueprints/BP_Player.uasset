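; Player pawn for an endless forward-flying game that dodges on two axes and fires rocks.
; Tick compounds forward speed every frame, even when dead, and applies a swept world-X offset while alive.
; Axis inputs feed swept local offsets through consumed movement input; left click spawns BP_Rock at the pawn's transform.
; It owns the HUD and restart widgets, with functions to show the restart screen and reset health, speed and score.
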(event `self.ReceiveBeginPlay`
  ;[1 1 1] Create widgets at start
  (bind _returnvalue (`|CreateWidget` "/Game/InfiniteMatrix/UI/WBP_Restart.WBP_Restart_C"))
  (set `self.RestartWidget` _returnvalue)
  (bind _returnvalue_2 (`|CreateWidget` "/Game/InfiniteMatrix/UI/WB_HUD.WB_HUD_C"))
  (`UserWidget.AddToViewport` _returnvalue_2 0)
  (set `self.HudWidget` _returnvalue_2))

(event `self.ReceiveTick`
  (params (DeltaSeconds :type "Float (single-precision)"))
  ;[0.07338 0.01239 1] Forward Movement (& projectile movement)
  (bind _output_get (set `self.ForwardSpeed` (* (`self.ForwardSpeed`) 1.0001)))
  (if (not (`self.IsDead`))
    (`self.K2_AddActorWorldOffset` (`KismetMathLibrary.MakeVector` (* DeltaSeconds _output_get)) true)))

(event `InputAxis|MoveUp`
  (params (AxisValue :type "Float (single-precision)"))
  ;[1 1 1] Horizontal and vertical movement
  (`self.AddMovementInput` (`self.GetActorUpVector`) (* AxisValue (`self.MoveSpeed`)))
  (bind _returnvalue (`self.ConsumeMovementInputVector` :!label _label))
  (`self.K2_AddActorLocalOffset` (* _returnvalue (`GameplayStatics.GetWorldDeltaSeconds`)) true))

(event `InputAxis|MoveRight`
  (params (AxisValue :type "Float (single-precision)"))
  ;[1 1 1] Horizontal and vertical movement
  (`self.AddMovementInput` (`self.GetActorRightVector`) (* AxisValue (`self.MoveSpeed`)))
  (goto _label))

(event `Key|LeftMouseButton`
  (params (Key :type "Key Structure"))
  ;[0 1 0.107] Projectile Handling
  (:`Pressed`
    (`|SpawnActorFromClass` "/Game/InfiniteMatrix/Blueprints/BP_Rock.BP_Rock_C" (`self.GetTransform`) "Undefined" "OverrideRootScale" null null)))

(fn `DisplayRestart`
  (bind _returnvalue (`GameplayStatics.GetPlayerController` 0))
  (bind _restartwidget (`self.RestartWidget`))
  (if (not (`Widget.IsInViewport` _restartwidget))
    (`UserWidget.AddToViewport` _restartwidget 0)
    (`WidgetBlueprintLibrary.SetInputMode_UIOnlyEx` _returnvalue null)
    (set `PlayerController.bShowMouseCursor` true _returnvalue)))

(fn `RestartGame`
  (bind _returnvalue (`GameplayStatics.GetPlayerController` 0))
  (bind _hudwidget (`self.HudWidget`))
  ;[1 1 1] Restart
  (set `self.IsDead` false)
  (`Widget.RemoveFromParent` (`self.RestartWidget`))
  (`WidgetBlueprintLibrary.SetInputMode_GameOnly` _returnvalue)
  (set `PlayerController.bShowMouseCursor` false _returnvalue)
  (bind _output_get (set `self.Health` 100.0))
  (`/Game/InfiniteMatrix/UI/WB_HUD.UpdateHealthbar` _hudwidget _output_get)
  (set `self.ForwardSpeed` 2000.0) ; Reset speed
  (bind _output_get_2 (set `self.Score` 0.0))
  (`/Game/InfiniteMatrix/UI/WB_HUD.UpdateScore` _hudwidget _output_get_2))

(fn `UserConstructionScript`)